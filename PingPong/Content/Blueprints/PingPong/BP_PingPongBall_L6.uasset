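; Ping-pong ball Blueprint that relays ball power and score changes to the player pawns.
; On BeginPlay it caches every BP_PingPongPlayerPawn and binds to its own power-change and score-change dispatchers.
; Each handler loops over the cached pawns, calling ChangeBallPower or RefreshScore with the score and gate ID.
; The score refresh always passes zero ball power, ignoring the dispatched value.
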(event `self.ReceiveBeginPlay`
  (bind _outactors (`GameplayStatics.GetAllActorsOfClass` "/Game/Blueprints/PingPong/BP_PingPongPlayerPawn.BP_PingPongPlayerPawn_C"))
  (set `self.Array` _outactors)
  (add `self.OnChangeBallPoewr` (delegate `OnChangeBallPoewr_Event_0`))
  (add `self.OnChageScore` (delegate `OnChageScore_Event_0`)))

(event `OnChangeBallPoewr_Event_0` :!signature `self.OnChangeBallPoewr`
  (params (BallPower :type Integer))
  (for _array_element (`self.Array`)
    (`/Game/Blueprints/PingPong/BP_PingPongPlayerPawn.ChangeBallPower` _array_element BallPower)))

(event `OnChageScore_Event_0` :!signature `self.OnChageScore`
  (params (Score :type Integer) (GateId :type Integer) (BallPower :type Integer))
  (for _array_element (`self.Array`)
    (`/Game/Blueprints/PingPong/BP_PingPongPlayerPawn.RefreshScore` _array_element Score GateId 0)))

(fn `UserConstructionScript`)