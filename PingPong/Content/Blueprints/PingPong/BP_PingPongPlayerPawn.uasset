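; BP_PingPongPlayerPawn is the player pawn for a ping pong game, and its graph handles the on-screen score display.
; On BeginPlay it creates a WBP_Score widget, keeps a reference to it and adds it to the viewport.
; Its RefreshScore event takes a score and an ID and writes the value to the widget's matching Gate1 or Gate2 text.
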(event `self.ReceiveBeginPlay`
  (bind _returnvalue (`|CreateWidget` "/Game/UI/WBP_Score.WBP_Score_C"))
  (bind _output_get (set `self.Score_Widget` _returnvalue))
  (`UserWidget.AddToViewport` _output_get 0))

(event `RefreshScore`
  (params (Score :type Integer) (ScoreID :type Integer))
  (if (== ScoreID 1)
    (`TextBlock.SetText` (`/Game/UI/WBP_Score.Gate1` (`self.Score_Widget`)) (`KismetTextLibrary.Conv_IntToText` Score))
    (elif (== ScoreID 2)
      (`TextBlock.SetText` (`/Game/UI/WBP_Score.Gate2` (`self.Score_Widget`)) (`KismetTextLibrary.Conv_IntToText` Score)))))

(fn `UserConstructionScript`)